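; PB_PickupItem is an item actor that a character picks up by overlapping it.
; On overlap it passes itself to the character's PB_PlayerState through PickupItem.
; If a SoundCue is set, it plays the sound at its location and dispatches its OnGet actions with the overlapping actor as trigger; without one, neither happens.
; The item destroys itself when its ItemAddedToInventory event fires.
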(event `self.ReceiveActorBeginOverlap`
  (params (OtherActor :type "Actor Object Reference"))
  (bind _soundcue (`self.SoundCue`))
  (bind _ascharacter (cast `Character` OtherActor))
  (bind _aspb_player_state (cast `/Game/PuzzleBox/Blueprints/Private/PB_PlayerState` (`Pawn.PlayerState` _ascharacter)))
  (`/Game/PuzzleBox/Blueprints/Private/PB_PlayerState.PickupItem` _aspb_player_state self)
  (`/Engine/EditorBlueprintResources/StandardMacros.IsValid` _soundcue
    (:`Is Valid`
      (`GameplayStatics.SpawnSoundAtLocation` _soundcue (`self.K2_GetActorLocation`) (struct) 1.0 1.0 0.0 null null)
      (`self.Dispatch` (`self.OnGet`) OtherActor))))

(event `ItemAddedToInventory`
  (`self.K2_DestroyActor`))

(fn `UserConstructionScript`)