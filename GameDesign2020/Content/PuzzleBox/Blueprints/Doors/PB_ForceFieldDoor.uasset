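; Force field door for PuzzleBox that opens by changing opacity and dropping collision.
; The construction script calls its parent, creates a dynamic material on the door mesh and applies the configurable color, pattern scale and pattern speed.
; OnUpdate takes an Alpha to blend between closed and opened opacity, disabling mesh collision past the halfway point and restoring it otherwise.
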(fn `OnUpdate`
  (params (Alpha :type "Float (double-precision)"))
  (bind _doormesh (`self.DoorMesh`))
  (`MaterialInstanceDynamic.SetScalarParameterValue` (`self.Material`) "Opacity" (`KismetMathLibrary.Lerp` (`self.ClosedOpacity`) (`self.OpenedOpacity`) Alpha))
  (if (> Alpha 0.5)
    (`PrimitiveComponent.SetCollisionEnabled` _doormesh "NoCollision")
    (else
      (`PrimitiveComponent.SetCollisionEnabled` _doormesh "QueryAndPhysics"))))

(fn `UserConstructionScript`
  (`parent.UserConstructionScript`)
  (bind _returnvalue (`PrimitiveComponent.CreateDynamicMaterialInstance` (`self.DoorMesh`) 0 null "None"))
  (set `self.Material` _returnvalue)
  (`MeshComponent.SetVectorParameterValueOnMaterials` (`self.DoorMesh`) "BaseColor" (`KismetMathLibrary.Conv_LinearColorToVector` (`KismetMathLibrary.Conv_ColorToLinearColor` (`self.Color`))))
  (`MeshComponent.SetScalarParameterValueOnMaterials` (`self.DoorMesh`) "PatternScale" (`self.PatternScale`))
  (`MeshComponent.SetScalarParameterValueOnMaterials` (`self.DoorMesh`) "PatternSpeed" (`self.PatternSpeed`)))