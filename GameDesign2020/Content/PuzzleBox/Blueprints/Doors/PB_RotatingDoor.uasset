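; PB_RotatingDoor is a puzzle box door Blueprint that swings open and closed by rotating around its yaw axis.
; Its update function maps the incoming alpha to an angle between minimum and maximum rotation, with a flip flag reversing the direction.
; That angle is combined with the start transform's rotation and applied to the actor, while the construction script only calls the parent's.
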(fn `OnUpdate`
  (params (Alpha :type "Float (double-precision)"))
  (`self.K2_SetActorRotation` (`KismetMathLibrary.ComposeRotators` (.rotation (`self.StartTransform`)) (`KismetMathLibrary.MakeRotator` 0.0 0.0 (* (`KismetMathLibrary.Lerp` (`self.MinimumRotation`) (`self.MaximumRotation`) Alpha) (`KismetMathLibrary.SelectFloat` -1.0 1.0 (`self.FlipRotation`)))))))

(fn `UserConstructionScript`
  (`parent.UserConstructionScript`))