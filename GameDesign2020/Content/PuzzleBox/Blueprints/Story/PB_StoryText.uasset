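; PB_StoryText is a PuzzleBox triggerable that sends a sequence of timed story segments to the triggering character's player state.
; On and toggle-on push the segments and play trigger sounds, stopping them after a delay equal to the summed segment times.
; Off and toggle-off flush the story from the player state.
; Only the on event checks Active, which is set true again afterwards unless OneShot.
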(event `self.TriggerOn`
  (params (TriggeringActor :type "Actor Object Reference") (Character :type "Character Object Reference"))
  (if (`self.active`)
    (bind _aspuzzle_player_state (`self.TryToGetPuzzlePlayerState` Character))
    (set `self.IsOn` true)
    (`/Game/PuzzleBox/Blueprints/Private/PB_PlayerState.NewStorySegments` _aspuzzle_player_state (`self.Story`))
    (`self.PlayTriggerSounds` true)
    (bind _duration (`self.GetStoryDuration` :!label _label))
    (`KismetSystemLibrary.Delay` _duration)
    (`self.StopTriggerSounds`)
    (if (not (`self.OneShot`)) :!label _label_2
      (set `self.active` true))))

(event `self.TriggerOff`
  (params (TriggeringActor :type "Actor Object Reference") (Character :type "Character Object Reference"))
  (bind _aspuzzle_player_state (`self.TryToGetPuzzlePlayerState` Character))
  (set `self.IsOn` false)
  (`/Game/PuzzleBox/Blueprints/Private/PB_PlayerState.StoryFlushed` _aspuzzle_player_state (`self.Story`))
  (`self.PlayTriggerSounds` false)
  (goto _label_2))

(event `self.TriggerToggle`
  (params (TriggeringActor :type "Actor Object Reference") (Character :type "Character Object Reference"))
  (bind _aspuzzle_player_state (`self.TryToGetPuzzlePlayerState` Character))
  (bind _output_get (set `self.IsOn` (not (`self.IsOn`))))
  (if _output_get
    (`/Game/PuzzleBox/Blueprints/Private/PB_PlayerState.NewStorySegments` _aspuzzle_player_state (`self.Story`))
    (`self.PlayTriggerSounds` true)
    (goto _label)
    (else
      (`/Game/PuzzleBox/Blueprints/Private/PB_PlayerState.StoryFlushed` _aspuzzle_player_state (`self.Story`))
      (`self.PlayTriggerSounds` false)
      (goto _label_2))))

(fn `GetStoryDuration`
  (returns (Duration :type "Float (double-precision)"))
  (locals (Seconds :type "Float (double-precision)"))
  (for _array_element (`self.Story`)
    (set `local.Seconds` (+ (`.Time_5_401C18EC4667157FECC25BB1BB61B5AB` (break `/Game/PuzzleBox/Blueprints/Private/PB_StorySegment` _array_element)) (`local.Seconds`))))
  (return (`local.Seconds`)))

(fn `UserConstructionScript`
  (`parent.UserConstructionScript`))