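; PuzzleBox component that plays a sound cue in response to trigger on and off events.
; TriggerOn and TriggerOff share one path, each gated by its own play flag, which spawns the cue attached to the component, stores the audio component and fades it in.
; Stop fades out the stored audio unless the sound is marked one-shot.
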(event `TriggerOn`
  (if (and (`self.PlayWhenTurnedOn`) (`KismetSystemLibrary.IsValid` (`self.SoundCue`)))
    (bind _returnvalue (`GameplayStatics.SpawnSoundAttached` (`self.SoundCue`) self "None" (0.0 0.0 0.0) (struct) "KeepRelativeOffset" true 1.0 1.0 0.0 null null :!label _label))
    (bind _output_get (set `self.AudioComponent` _returnvalue))
    (`AudioComponent.FadeIn` _output_get (`self.FadeInTime`) 1.0 0.0 "Linear")))

(event `TriggerOff`
  (if (and (`self.PlayWhenTurnedOff`) (`KismetSystemLibrary.IsValid` (`self.SoundCue`)))
    (goto _label)))

(event `Stop`
  (if (and (not (`self.OneShot`)) (`KismetSystemLibrary.IsValid` (`self.AudioComponent`)))
    (`AudioComponent.FadeOut` (`self.AudioComponent`) (`self.FadeOutTime`) 0.0 "Linear")))