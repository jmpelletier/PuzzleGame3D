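; Puzzle box trigger that ends the game as cleared for the character that activates it.
; On trigger, it marks the game clear on the PB player state, plays trigger sounds and pauses the player through the PB player controller.
; OnGameClear then binds an event to the controller's left click, alongside a ReloadLevel function that reopens the current level by name.
; The trigger off and toggle events are empty.
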(event `self.TriggerOn`
  (params (TriggeringActor :type "Actor Object Reference") (Character :type "Character Object Reference"))
  (`/Engine/EditorBlueprintResources/StandardMacros.IsValid` Character
    (:`Is Valid`
      (bind _aspb_player_state (cast `/Game/PuzzleBox/Blueprints/Private/PB_PlayerState` (`Pawn.PlayerState` Character)))
      (`/Game/PuzzleBox/Blueprints/Private/PB_PlayerState.GameClear` _aspb_player_state)
      (`self.PlayTriggerSounds` true)
      (bind _aspb_player_controller (cast `/Game/PuzzleBox/Blueprints/Private/PB_PlayerController` (`Pawn.GetController` Character)))
      (`/Game/PuzzleBox/Blueprints/Private/PB_PlayerController.PausePlayer` _aspb_player_controller)
      (`self.OnGameClear` _aspb_player_controller))))

(event `self.TriggerOff`
  (params (TriggeringActor :type "Actor Object Reference") (Character :type "Character Object Reference")))

(event `self.TriggerToggle`
  (params (TriggeringActor :type "Actor Object Reference") (Character :type "Character Object Reference")))

(fn `OnGameClear`
  (params (PlayerController :type "/Game/PuzzleBox/Blueprints/Private/PB_PlayerController Object Reference"))
  (add `/Game/PuzzleBox/Blueprints/Private/PB_PlayerController.OnLeftClick` PlayerController (`|CreateDelegate` :!event `ReloadLevel`)))

(fn `ReloadLevel`
  (bind _returnvalue (`GameplayStatics.GetCurrentLevelName` true))
  (`GameplayStatics.OpenLevel` (`KismetStringLibrary.Conv_StringToName` _returnvalue)))

(fn `UserConstructionScript`
  (`parent.UserConstructionScript`))