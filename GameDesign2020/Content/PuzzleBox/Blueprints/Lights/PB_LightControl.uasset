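; Puzzle light controller that fades its light components on and off in response to on, off and toggle triggers, with trigger sounds.
; On BeginPlay it uses assigned lights or gathers its own, caches their intensities, and starts on or off via StartOff.
; One timeline scales cached intensities and hides lights at zero.
; It plays forward or in reverse at rates from OnTime and OffTime, and toggle flips its last direction.
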(event `self.ReceiveBeginPlay`
  (bind _intensitytimeline (`self.IntensityTimeline`))
  (`parent.ReceiveBeginPlay`)
  (bind _lights (`self.GetLights`)
    (:`Found Light`
      (for _array_element _lights
        (`BlueprintMapLibrary.Map_Add` (`self.Intensities`) _array_element (`LightComponentBase.Intensity` _array_element)))
      (if (`self.StartOff`)
        (set `self.Direction` "Backward")
        (`TimelineComponent.SetPlaybackPosition` _intensitytimeline 0.0 false true)
        (bind (_direction _intensity) (`Timeline|IntensityTimeline` :!via `Reverse` :!label _label)
          (:`Update`
            (set `self.Direction` _direction)
            (for _array_element_2 (`self.LightComponents`)
              (bind (_value _returnvalue) (`BlueprintMapLibrary.Map_Find` (`self.Intensities`) _array_element_2))
              (if _returnvalue
                (bind _returnvalue_2 (* _value _intensity))
                (`LightComponent.SetIntensity` _array_element_2 _returnvalue_2)
                (`SceneComponent.SetVisibility` _array_element_2 (> _returnvalue_2 0.0) false))))
          (:`Finished`
            (`self.StopTriggerSounds`)))
        (else
          (set `self.Direction` "Forward")
          (`TimelineComponent.SetPlaybackPosition` _intensitytimeline 1.0 false true)
          (goto _label))))))

(event `self.TriggerOn`
  (params (TriggeringActor :type "Actor Object Reference") (Character :type "Character Object Reference"))
  (`TimelineComponent.SetPlayRate` (`self.IntensityTimeline`) (`self.TimeToRate` (`self.OnTime`)) :!label _label_2)
  (`self.PlayTriggerSounds` true)
  (goto _label))

(event `self.TriggerOff`
  (params (TriggeringActor :type "Actor Object Reference") (Character :type "Character Object Reference"))
  (`TimelineComponent.SetPlayRate` (`self.IntensityTimeline`) (`self.TimeToRate` (`self.OffTime`)) :!label _label_3)
  (`self.PlayTriggerSounds` false)
  (goto _label :!via `Reverse`))

(event `self.TriggerToggle`
  (params (TriggeringActor :type "Actor Object Reference") (Character :type "Character Object Reference"))
  (switch `ETimelineDirection` (`self.Direction`)
    (:`Forward`
      (goto _label_3))
    (:`Backward`
      (goto _label_2))))

(fn `UserConstructionScript`
  (`parent.UserConstructionScript`))