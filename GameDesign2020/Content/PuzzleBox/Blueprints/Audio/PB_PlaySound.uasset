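; PB_PlaySound is a PuzzleBox audio Blueprint that starts and stops a sound through trigger events.
; Trigger on plays its Audio component with a fade-in; trigger off fades out linearly, then stops it after the fade time.
; Both paths act only when a sound is assigned.
; Toggle reuses both paths but looks inverted: it runs the play path when already playing and the stop path otherwise.
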(event `self.TriggerOn`
  (params (TriggeringActor :type "Actor Object Reference") (Character :type "Character Object Reference"))
  (bind _audio (`self.Audio`))
  (`/Engine/EditorBlueprintResources/StandardMacros.IsValid` (`AudioComponent.Sound` (`self.Audio`)) :!label _label
    (:`Is Valid`
      (`AudioComponent.Play` _audio 0.0)
      (`AudioComponent.FadeIn` _audio (`self.FadeInTime`) 1.0 0.0 "Linear"))))

(event `self.TriggerOff`
  (params (TriggeringActor :type "Actor Object Reference") (Character :type "Character Object Reference"))
  (bind _audio (`self.Audio`))
  (bind _fadeouttime (`self.FadeOutTime`))
  (`/Engine/EditorBlueprintResources/StandardMacros.IsValid` (`AudioComponent.Sound` (`self.Audio`)) :!label _label_2
    (:`Is Valid`
      (`AudioComponent.FadeOut` _audio _fadeouttime 0.0 "Linear")
      (`AudioComponent.StopDelayed` _audio _fadeouttime))))

(event `self.TriggerToggle`
  (params (TriggeringActor :type "Actor Object Reference") (Character :type "Character Object Reference"))
  (if (`AudioComponent.IsPlaying` (`self.Audio`))
    (goto _label)
    (else
      (goto _label_2))))

(fn `UserConstructionScript`
  (`parent.UserConstructionScript`))