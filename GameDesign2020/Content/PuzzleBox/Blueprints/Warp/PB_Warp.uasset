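; PuzzleBox warp actor that, when triggered while active, teleports either the triggering actor or the character to its own transform, as set by Mode.
; It aligns control rotation for pawns or actor rotation otherwise, and redirects velocity along its forward vector, preserving speed.
; Before moving the target, it temporarily deactivates its paired warp with a retriggerable delay and plays trigger sounds.
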(event `self.TriggerOn`
  (params (TriggeringActor :type "Actor Object Reference") (Character :type "Character Object Reference"))
  (bind _target (`self.Target`))
  (bind _pair (`self.Pair`))
  (bind _rotation (.rotation (`self.GetTransform`)))
  (bind _returnvalue (`self.GetComponentByClass` _target "/Script/Engine.MovementComponent"))
  (if (`self.Active`)
    (switch `/Game/PuzzleBox/Blueprints/Private/PB_TeleportModes` (`self.Mode`)
      (:`NewEnumerator0`
        (set `self.Target` TriggeringActor))
      (:`NewEnumerator1`
        (set `self.Target` Character)))
    (`/Engine/EditorBlueprintResources/StandardMacros.IsValid` (`self.Target`)
      (:`Is Valid`
        (`/Engine/EditorBlueprintResources/StandardMacros.IsValid` _pair
          (:`Is Valid`
            (`self.WaitForTransit` _pair))
          (:`Is Not Valid`
            _))
        (`self.PlayTriggerSounds` true)
        (`self.K2_SetActorLocation` _target (.location (`self.GetTransform`)) false true)
        (bind _aspawn (cast `Pawn` _target)
          (:`then`
            (`Controller.SetControlRotation` (`Pawn.GetController` _aspawn) _rotation))
          (:`CastFailed`
            (`self.K2_SetActorRotation` _target _rotation true)))
        (`/Engine/EditorBlueprintResources/StandardMacros.IsValid` _returnvalue
          (:`Is Valid`
            (set `MovementComponent.Velocity` (* (`KismetMathLibrary.GetForwardVector` _rotation) (`KismetMathLibrary.VSize` (`self.GetVelocity` _target))) _returnvalue)))))))

(event `WaitForTransit`
  (set `self.Active` false)
  (`KismetSystemLibrary.RetriggerableDelay` (`self.PairFreezeTime`))
  (set `self.Active` true))

(fn `UserConstructionScript`
  (`parent.UserConstructionScript`))