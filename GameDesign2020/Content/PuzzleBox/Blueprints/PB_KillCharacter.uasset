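; PuzzleBox triggerable Blueprint that kills the player character passed to its trigger-on event.
; It casts the character's controller to PB_PlayerController and, if the player is alive, plays trigger sounds and calls KillPlayer.
; OnPlayerKilled then binds an event to the controller's left click, and a ReloadLevel function reopens the current level by name.
; The trigger-off and toggle events do nothing.
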(event `self.TriggerOn`
  (params (TriggeringActor :type "Actor Object Reference") (Character :type "Character Object Reference"))
  (`/Engine/EditorBlueprintResources/StandardMacros.IsValid` Character
    (:`Is Valid`
      (bind _aspb_player_controller (cast `/Game/PuzzleBox/Blueprints/Private/PB_PlayerController` (`Pawn.GetController` Character)))
      (bind _alive (`/Game/PuzzleBox/Blueprints/Private/PB_PlayerController.IsAlive` _aspb_player_controller))
      (if _alive
        (`self.PlayTriggerSounds` true)
        (`/Game/PuzzleBox/Blueprints/Private/PB_PlayerController.KillPlayer` _aspb_player_controller)
        (`self.OnPlayerKilled` _aspb_player_controller)))))

(event `self.TriggerOff`
  (params (TriggeringActor :type "Actor Object Reference") (Character :type "Character Object Reference")))

(event `self.TriggerToggle`
  (params (TriggeringActor :type "Actor Object Reference") (Character :type "Character Object Reference")))

(fn `OnPlayerKilled`
  (params (PlayerController :type "/Game/PuzzleBox/Blueprints/Private/PB_PlayerController Object Reference"))
  (add `/Game/PuzzleBox/Blueprints/Private/PB_PlayerController.OnLeftClick` PlayerController (`|CreateDelegate` :!event `ReloadLevel`)))

(fn `ReloadLevel`
  (bind _returnvalue (`GameplayStatics.GetCurrentLevelName` true))
  (`GameplayStatics.OpenLevel` (`KismetStringLibrary.Conv_StringToName` _returnvalue)))

(fn `UserConstructionScript`
  (`parent.UserConstructionScript`))