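; PuzzleBox player state that tracks whether the player is alive, active timers and picked-up items.
; On BeginPlay it sets game-only input, adds the PB player control component to its pawn and announces the spawn.
; Events for death, game clear, timer start or stop, pickups and story segments update any related state, then relay it through Call notifications.
; Timer notifications fire only when the active list actually changes.
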(event `GameClear`
  (`self.GameCleared`))

(event `KillPlayer`
  (set `self.Alive` false)
  (`self.PlayerDied`))

(event `self.ReceiveBeginPlay`
  (bind _pawnprivate (`self.PawnPrivate`))
  (bind _asplayer_controller (cast `PlayerController` (`Pawn.GetController` _pawnprivate)))
  (`WidgetBlueprintLibrary.SetInputMode_GameOnly` _asplayer_controller)
  (`AddComponent|NODE_AddPlayerDeathComponent-0` :`self` _pawnprivate)
  (set `self.Alive` true)
  (`self.PlayerSpawned`))

(event `StartTimer`
  (params (Timer :type "/Game/PuzzleBox/Blueprints/Triggers/PB_TimerTrigger Object Reference"))
  (bind _returnvalue (`KismetArrayLibrary.Array_AddUnique` (`self.ActiveTimers`) Timer))
  (if (!= _returnvalue -1)
    (`self.TimerStarted` Timer)))

(event `StopTimer`
  (params (Timer :type "/Game/PuzzleBox/Blueprints/Triggers/PB_TimerTrigger Object Reference"))
  (bind _activetimers (`self.ActiveTimers`))
  (bind _returnvalue (`KismetArrayLibrary.Array_Find` _activetimers Timer))
  (if (!= _returnvalue -1)
    (`KismetArrayLibrary.Array_Remove` _activetimers _returnvalue)
    (`self.TimerCanceled` Timer)))

(event `PickupItem`
  (params (Item :type "/Game/PuzzleBox/Blueprints/Items/PB_PickupItem Object Reference"))
  (`KismetArrayLibrary.Array_Add` (`self.PickupItems`) Item)
  (`self.PickedUpItem` Item))

(event `NewStorySegments`
  (params (Segments :type "Array of /Game/PuzzleBox/Blueprints/Private/PB_StorySegment Structure"))
  (`self.StoryUpdated` Segments))

(event `FlushStorySegments`
  (params (Segments :type "Array of /Game/PuzzleBox/Blueprints/Private/PB_StorySegment Structure"))
  (`self.StoryFlushed` Segments))

(fn `UserConstructionScript`)