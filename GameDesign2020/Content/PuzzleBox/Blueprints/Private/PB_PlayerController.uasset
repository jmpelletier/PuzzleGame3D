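; Puzzle Box player controller that handles player death and pausing, and broadcasts left-click releases.
; KillPlayer disables input and movement, freezes animation, then notifies PB_PlayerState, whose Alive flag gates both events.
; Death uses physics: a first-person branch shrinks and topples the capsule with an angular impulse, while other characters ragdoll their mesh.
; PausePlayer stops input and movement but sets PauseAnims to false, leaving animation running.
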(event `KillPlayer`
  (bind _pawnprivate (`PlayerState.PawnPrivate` (`self.PlayerState`)))
  (bind _returnvalue (`GameplayStatics.GetObjectClass` (`PlayerState.PawnPrivate` (`self.PlayerState`))))
  (bind _alive (`self.IsAlive`))
  (if _alive
    (`self.DisableInput` _pawnprivate self)
    (`MovementComponent.StopMovementImmediately` (`Pawn.GetMovementComponent` _pawnprivate))
    (bind _mesh (`self.Get Animation Mesh` _pawnprivate))
    (set `SkeletalMeshComponent.bPauseAnims` true _mesh)
    (bind _ascharacter (cast `Character` (`PlayerState.PawnPrivate` (`self.PlayerState`))))
    (if (or (== _returnvalue "/Game/PuzzleBox/Blueprints/Characters/PB_FirstPersonCharacter.PB_FirstPersonCharacter_C") (== _returnvalue "/Game/FirstPersonBP/Blueprints/FirstPersonCharacter.FirstPersonCharacter_C"))
      (bind _capsulecomponent (`Character.CapsuleComponent` _ascharacter))
      (`PrimitiveComponent.SetSimulatePhysics` _capsulecomponent true)
      (`CapsuleComponent.SetCapsuleSize` _capsulecomponent 15.0 15.0 true)
      (`PrimitiveComponent.SetPhysicsLinearVelocity` _capsulecomponent (0.0 0.0 0.0) false "None")
      (bind _returnvalue_2 (`self.GetComponentByClass` _ascharacter "/Script/Engine.CameraComponent"))
      (set `CameraComponent.bUsePawnControlRotation` false _returnvalue_2)
      (`PrimitiveComponent.AddAngularImpulseInRadians` _capsulecomponent (* (`KismetMathLibrary.Spherical2DToUnitCartesian` (+ (`KismetMathLibrary.Vector_UnitCartesianToSpherical` (`SceneComponent.GetForwardVector` _returnvalue_2)) (3.1416 0.0))) 0.2) "None" true)
      (`PrimitiveComponent.SetAngularDamping` _capsulecomponent 0.9)
      (`PrimitiveComponent.SetPhysicsMaxAngularVelocityInDegrees` _capsulecomponent 30.0 false "None")
      (else
        (`PrimitiveComponent.SetCollisionEnabled` _capsulecomponent "QueryOnly")
        (bind _mesh_2 (`Character.Mesh` _ascharacter))
        (`PrimitiveComponent.SetSimulatePhysics` _mesh_2 true)
        (`PrimitiveComponent.SetCollisionProfileName` _mesh_2 "PhysicsActor")))
    (bind _aspb_player_state (cast `/Game/PuzzleBox/Blueprints/Private/PB_PlayerState` (`self.PlayerState`)))
    (`/Game/PuzzleBox/Blueprints/Private/PB_PlayerState.KillPlayer` _aspb_player_state)))

(event `PausePlayer`
  (bind _pawnprivate (`PlayerState.PawnPrivate` (`self.PlayerState`)))
  (bind _alive (`self.IsAlive`))
  (if _alive
    (`self.DisableInput` (`PlayerState.PawnPrivate` (`self.PlayerState`)) self)
    (`MovementComponent.StopMovementImmediately` (`Pawn.GetMovementComponent` _pawnprivate))
    (bind _mesh (`self.Get Animation Mesh` _pawnprivate))
    (set `SkeletalMeshComponent.bPauseAnims` false _mesh)))

(event `Key|LeftMouseButton` :consume false
  (params (Key :type "Key Structure"))
  (:`Released`
    (`self.OnLeftClick`)))

(fn `Get Animation Mesh`
  (params (Pawn :type "Pawn Object Reference"))
  (returns (Mesh :type "SkeletalMeshComponent Object Reference"))
  (bind _aspb_first_person_character (cast `/Game/PuzzleBox/Blueprints/Characters/PB_FirstPersonCharacter` Pawn)
    (:`then`
      (return (`/Game/PuzzleBox/Blueprints/Characters/PB_FirstPersonCharacter.Mesh2P` _aspb_first_person_character)))
    (:`CastFailed`
      (bind _asfirst_person_character (cast `/Game/FirstPersonBP/Blueprints/FirstPersonCharacter` Pawn)
        (:`then`
          (return (`/Game/FirstPersonBP/Blueprints/FirstPersonCharacter.Mesh2P` _asfirst_person_character)))
        (:`CastFailed`
          (bind _ascharacter (cast `Character` Pawn))
          (return (`Character.Mesh` _ascharacter)))))))

(fn `IsAlive`
  (returns (Alive :type Boolean))
  (bind _aspb_player_state (cast `/Game/PuzzleBox/Blueprints/Private/PB_PlayerState` (`self.PlayerState`))
    (:`then`
      (return (`/Game/PuzzleBox/Blueprints/Private/PB_PlayerState.Alive` _aspb_player_state)))
    (:`CastFailed`
      (return false))))

(fn `UserConstructionScript`)