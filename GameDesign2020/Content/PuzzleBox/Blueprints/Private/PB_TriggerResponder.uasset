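; Base actor for PuzzleBox objects that respond to triggers, with empty TriggerOn, TriggerOff and TriggerToggle events that receive the triggering actor and character.
; On BeginPlay it caches its PB_TriggerSoundComponents.
; Helper functions switch those sounds on or off by state or stop them all, and can spawn a sound cue attached to the Scene component that stops when that component is destroyed.
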(event `TriggerOn`
  (params (TriggeringActor :type "Actor Object Reference") (Character :type "Character Object Reference")))

(event `TriggerOff`
  (params (TriggeringActor :type "Actor Object Reference") (Character :type "Character Object Reference")))

(event `TriggerToggle`
  (params (TriggeringActor :type "Actor Object Reference") (Character :type "Character Object Reference")))

(event `self.ReceiveBeginPlay`
  (set `self.TriggerSounds` (`self.K2_GetComponentsByClass` "/Game/PuzzleBox/Blueprints/Components/PB_TriggerSoundComponent.PB_TriggerSoundComponent_C")))

(fn `PlayTriggerSounds`
  (params (State :type Boolean))
  (for _array_element (`self.TriggerSounds`)
    (if State
      (`/Game/PuzzleBox/Blueprints/Components/PB_TriggerSoundComponent.TriggerOn` _array_element)
      (else
        (`/Game/PuzzleBox/Blueprints/Components/PB_TriggerSoundComponent.TriggerOff` _array_element)))))

(fn `StopTriggerSounds`
  (for _array_element (`self.TriggerSounds`)
    (`/Game/PuzzleBox/Blueprints/Components/PB_TriggerSoundComponent.Stop` _array_element)))

(fn `UserConstructionScript`)