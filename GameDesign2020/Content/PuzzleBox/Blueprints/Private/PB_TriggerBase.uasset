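; PB_TriggerBase is the base actor for PuzzleBox triggers, holding an Active state and the actor and Character that triggered it.
; On, Off and Toggle events update that state and call the empty StateChanged hook, though Toggle only acts while active.
; While active, Dispatch relays On, Off or Toggle actions to target actors.
; GetCharacter resolves the instigating Character directly or from an upstream trigger, carrying it along chains.
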(event `self.TriggerOn`
  (params (TriggeringActor :type "Actor Object Reference") (Character :type "Character Object Reference"))
  (set `self.TriggeringActor` TriggeringActor)
  (set `self.TriggeringCharacter` Character)
  (if (not (`self.Active`))
    (set `self.Active` true)
    (`self.StateChanged` :!label _label)))

(event `self.TriggerOff`
  (params (TriggeringActor :type "Actor Object Reference") (Character :type "Character Object Reference"))
  (set `self.TriggeringActor` TriggeringActor)
  (set `self.TriggeringCharacter` Character)
  (if (`self.Active`)
    (set `self.Active` false)
    (goto _label)))

(event `self.TriggerToggle`
  (params (TriggeringActor :type "Actor Object Reference") (Character :type "Character Object Reference"))
  (bind _active (`self.Active`))
  (set `self.TriggeringActor` TriggeringActor)
  (set `self.TriggeringCharacter` Character)
  (if _active
    (set `self.Active` (not _active))
    (goto _label)))

(fn `Dispatch`
  (params (Actions :type "Array of /Game/PuzzleBox/Blueprints/Private/PB_TriggerTargetAction Structure") (TriggeringActor :type "Actor Object Reference"))
  (locals (old_state :type Boolean) (TargetActor :type "/Game/PuzzleBox/Blueprints/Private/PB_TriggerResponder Object Reference"))
  (bind _triggeringactor (`local.TriggeringActor`))
  (bind _triggeringcharacter (`self.TriggeringCharacter`))
  (bind _targetactor (`local.TargetActor`))
  (if (`self.Active`)
    (bind _output_get (set `self.TriggeringActor` TriggeringActor))
    (bind _character (`self.GetCharacter` _output_get))
    (set `self.TriggeringCharacter` _character)
    (for _array_element Actions
      (bind (_actor _action) (break `/Game/PuzzleBox/Blueprints/Private/PB_TriggerTargetAction` _array_element))
      (`/Engine/EditorBlueprintResources/StandardMacros.IsValid` _actor
        (:`Is Valid`
          (set `local.TargetActor` _actor)
          (switch `/Game/PuzzleBox/Blueprints/Private/PB_TriggerActions` _action
            (:`NewEnumerator2`
              (`self.TriggerOn` _targetactor _triggeringactor _triggeringcharacter))
            (:`NewEnumerator3`
              (`self.TriggerOff` _targetactor _triggeringactor _triggeringcharacter))
            (:`NewEnumerator4`
              (`self.TriggerToggle` _targetactor _triggeringactor _triggeringcharacter))))))))

(fn `GetCharacter`
  (params (TriggeringActor :type "Actor Object Reference"))
  (returns (Character :type "Character Object Reference"))
  (bind _ascharacter (cast `Character` TriggeringActor)
    (:`then`
      (return _ascharacter))
    (:`CastFailed`
      (bind _aspb_trigger_base (cast `/Game/PuzzleBox/Blueprints/Private/PB_TriggerBase` TriggeringActor))
      (return (`/Game/PuzzleBox/Blueprints/Private/PB_TriggerResponder.TriggeringCharacter` _aspb_trigger_base)))))

(fn `StateChanged`)

(fn `UserConstructionScript`)