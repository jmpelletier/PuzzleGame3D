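; Keyed trigger for PuzzleBox that decides whether a given actor counts as a key, with no event logic of its own.
; ActorIsKey accepts actors listed in KeyActors outright, otherwise requires a class deriving from one of KeyClasses.
; Class-matched Characters also need every InventoryKeys entry in their PB_PlayerState PickupItems.
; Characters without a PB_PlayerState skip that inventory check and pass.
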(fn `Actor Is Key`
  (params (Actor :type "Actor Object Reference"))
  (returns (IsKey :type Boolean))
  (`self.ActorIsKeyActor` Actor
    (:`True`
      (return true))
    (:`False`
      (bind _haskeyclass (`self.ActorHasKeyClass` Actor))
      (if _haskeyclass
        (bind _ascharacter (cast `Character` Actor)
          (:`then`
            (bind _iskey (`self.CharacterIsKey` _ascharacter))
            (return _iskey))
          (:`CastFailed`
            (return true)))
        (else
          (return false))))))

(fn `ActorHasKeyClass`
  (params (Actor :type "Actor Object Reference"))
  (returns (HasKeyClass :type Boolean))
  (bind _result (`BlueprintSetLibrary.Set_ToArray` (`self.KeyClasses`)))
  (for _array_element _result
    (if (`KismetMathLibrary.ClassIsChildOf` (`GameplayStatics.GetObjectClass` Actor) _array_element)
      (return true)))
  (return false))

(fn `CharacterIsKey`
  (params (Character :type "Character Object Reference"))
  (returns (IsKey :type Boolean))
  (bind _aspb_player_state (cast `/Game/PuzzleBox/Blueprints/Private/PB_PlayerState` (`Pawn.PlayerState` Character))
    (:`then`
      (for _array_element (`self.InventoryKeys`)
        (if (not (`KismetArrayLibrary.Array_Contains` (`/Game/PuzzleBox/Blueprints/Private/PB_PlayerState.PickupItems` _aspb_player_state) _array_element))
          (return false))))
    (:`CastFailed`
      _))
  (return true))

(fn `UserConstructionScript`
  (`parent.UserConstructionScript`))