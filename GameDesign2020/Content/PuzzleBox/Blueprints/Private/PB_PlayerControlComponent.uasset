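; PuzzleBox player control component that kills or pauses its owning Character.
; Both events switch input to UI-only, stop movement and set animation pausing; pausing also unpossesses.
; Killing requires a living PB_PlayerState, which it then marks dead.
; First-person deaths shrink the capsule into a physics sphere and gently roll it with the released camera to fake collapsing, while other characters ragdoll their mesh and get unpossessed.
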(event `KillPlayer`
  (bind _alive (`self.OwnerIsAlive`))
  (if _alive
    (`self.FreezePlayer` true)
    (bind _character (`self.GetCharacter`))
    (bind _asfirst_person_character (cast `/Game/FirstPersonBP/Blueprints/FirstPersonCharacter` _character)
      (:`then`
        (`self.KillFirstPersonPlayer` _asfirst_person_character)
        (bind _playerstate (`self.GetPlayerState` :!label _label))
        (`/Game/PuzzleBox/Blueprints/Private/PB_PlayerState.KillPlayer` _playerstate))
      (:`CastFailed`
        (bind _aspb_first_person_character (cast `/Game/PuzzleBox/Blueprints/Characters/PB_FirstPersonCharacter` _character)
          (:`then`
            (`self.KillFirstPersonPlayer` _aspb_first_person_character)
            (goto _label))
          (:`CastFailed`
            (`self.KillThirdPersonPlayer` _character)
            (bind _playerstate_2 (`self.GetPlayerState`))
            (`/Game/PuzzleBox/Blueprints/Private/PB_PlayerState.KillPlayer` _playerstate_2)
            (bind _playercontroller (`self.GetPlayerController`))
            (`Controller.UnPossess` _playercontroller)))))))

(event `PausePlayer`
  (`self.FreezePlayer` false)
  (bind _playercontroller (`self.GetPlayerController`))
  (`Controller.UnPossess` _playercontroller))

(fn `FreezePlayer`
  (params (StopAnimations :type Boolean))
  (bind _playercontroller (`self.GetPlayerController`))
  (`Controller.SetIgnoreMoveInput` _playercontroller true)
  (`WidgetBlueprintLibrary.SetInputMode_UIOnlyEx` _playercontroller null)
  (bind _character (`self.GetCharacter`))
  (`MovementComponent.StopMovementImmediately` (`Pawn.GetMovementComponent` _character))
  (bind _mesh (`self.GetAnimationMesh` _character))
  (set `SkeletalMeshComponent.bPauseAnims` StopAnimations _mesh)
  (return))

(fn `Get FPCamera`
  (params (Character :type "Character Object Reference"))
  (returns (Camera :type "CameraComponent Object Reference"))
  (bind _asfirst_person_character (cast `/Game/FirstPersonBP/Blueprints/FirstPersonCharacter` Character)
    (:`then`
      (return (`/Game/FirstPersonBP/Blueprints/FirstPersonCharacter.FirstPersonCamera` _asfirst_person_character)))
    (:`CastFailed`
      (bind _aspb_first_person_character (cast `/Game/PuzzleBox/Blueprints/Characters/PB_FirstPersonCharacter` Character))
      (return (`/Game/PuzzleBox/Blueprints/Characters/PB_FirstPersonCharacter.FirstPersonCamera` _aspb_first_person_character)))))

(fn `GetAnimationMesh`
  (params (Character :type "Character Object Reference"))
  (returns (Mesh :type "SkeletalMeshComponent Object Reference"))
  (bind _asfirst_person_character (cast `/Game/FirstPersonBP/Blueprints/FirstPersonCharacter` Character)
    (:`then`
      (return (`/Game/FirstPersonBP/Blueprints/FirstPersonCharacter.Mesh2P` _asfirst_person_character)))
    (:`CastFailed`
      (bind _aspb_first_person_character (cast `/Game/PuzzleBox/Blueprints/Characters/PB_FirstPersonCharacter` Character)
        (:`then`
          (return (`/Game/PuzzleBox/Blueprints/Characters/PB_FirstPersonCharacter.Mesh2P` _aspb_first_person_character)))
        (:`CastFailed`
          (return (`Character.Mesh` Character)))))))

(fn `GetCharacter`
  (returns (Character :type "Character Object Reference"))
  (bind _ascharacter (cast `Character` (`self.GetOwner`)))
  (return _ascharacter))

(fn `GetPlayerController`
  (returns (PlayerController :type "PlayerController Object Reference"))
  (bind _aspawn (cast `Pawn` (`self.GetOwner`)))
  (bind _asplayer_controller (cast `PlayerController` (`Pawn.GetController` _aspawn)))
  (return _asplayer_controller))

(fn `GetPlayerState`
  (returns (PlayerState :type "/Game/PuzzleBox/Blueprints/Private/PB_PlayerState Object Reference"))
  (bind _aspawn (cast `Pawn` (`self.GetOwner`)))
  (bind _aspb_player_state (cast `/Game/PuzzleBox/Blueprints/Private/PB_PlayerState` (`Pawn.PlayerState` _aspawn)))
  (return _aspb_player_state))

(fn `KillFirstPersonPlayer`
  (params (Character :type "Character Object Reference"))
  (bind _capsulecomponent (`Character.CapsuleComponent` Character))
  ;[1 1 1] 物理計算をオンにする
  (`PrimitiveComponent.SetSimulatePhysics` _capsulecomponent true)
  ;[1 1 1] 転がしたいのでキャプセルを球体にする。
  (`CapsuleComponent.SetCapsuleSize` _capsulecomponent 15.0 15.0 true)
  ;[1 1 1] 動きを止める。
  (`PrimitiveComponent.SetPhysicsLinearVelocity` _capsulecomponent (0.0 0.0 0.0) false "None")
  (bind _camera (`self.Get FPCamera` Character))
  ;[1 1 1] 横たわるようにカメラが向いている方向を軸に穏やかに回転させる。
  ;;[1 1 1] カメラの回転を開放する
  (set `CameraComponent.bUsePawnControlRotation` false _camera)
  (`PrimitiveComponent.AddAngularImpulseInRadians` _capsulecomponent (* (`KismetMathLibrary.Spherical2DToUnitCartesian` (+ (`KismetMathLibrary.Vector_UnitCartesianToSpherical` (`SceneComponent.GetForwardVector` _camera)) (3.1416 0.0))) 0.2) "None" true)
  (`PrimitiveComponent.SetAngularDamping` _capsulecomponent 0.9)
  (`PrimitiveComponent.SetPhysicsMaxAngularVelocityInDegrees` _capsulecomponent 30.0 false "None")
  (return))

(fn `KillThirdPersonPlayer`
  (params (Character :type "Character Object Reference"))
  (bind _mesh (`Character.Mesh` Character))
  (`PrimitiveComponent.SetCollisionEnabled` (`Character.CapsuleComponent` Character) "QueryOnly")
  (`PrimitiveComponent.SetSimulatePhysics` _mesh true)
  (`PrimitiveComponent.SetCollisionProfileName` _mesh "PhysicsActor"))

(fn `OwnerIsAlive`
  (returns (Alive :type Boolean))
  (bind _aspawn (cast `Pawn` (`self.GetOwner`))
    (:`then`
      (bind _aspb_player_state (cast `/Game/PuzzleBox/Blueprints/Private/PB_PlayerState` (`Pawn.PlayerState` _aspawn))
        (:`then`
          (return (`/Game/PuzzleBox/Blueprints/Private/PB_PlayerState.Alive` _aspb_player_state)))
        (:`CastFailed`
          _)))
    (:`CastFailed`
      _))
  (return false))