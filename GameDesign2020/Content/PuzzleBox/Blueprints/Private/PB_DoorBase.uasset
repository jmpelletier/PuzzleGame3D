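; Base Blueprint for PuzzleBox doors that open and close in response to trigger on, off and toggle events.
; A timeline plays or reverses with its rate derived from OpenTime or CloseTime, while toggle picks the way from the last Direction.
; Each update passes Alpha to an empty OnUpdate hook, leaving the actual motion to child classes.
; BeginPlay caches the start transform and jumps the timeline to its end when StartOpen is set.
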(event `self.TriggerOn`
  (params (TriggeringActor :type "Actor Object Reference") (Character :type "Character Object Reference"))
  (`TimelineComponent.SetPlayRate` (`self.DoorTimeline`) (/ 1.0 (`KismetMathLibrary.FMax` (`self.OpenTime`) 0.008)) :!label _label)
  (`self.PlayTriggerSounds` true)
  (bind (_direction _alpha) (`Timeline|DoorTimeline` :!label _label_2)
    (:`Update`
      (set `self.Direction` _direction)
      (`self.OnUpdate` _alpha))
    (:`Finished`
      (`self.StopTriggerSounds`))))

(event `self.TriggerToggle`
  (params (TriggeringActor :type "Actor Object Reference") (Character :type "Character Object Reference"))
  (switch `ETimelineDirection` (`self.Direction`)
    (:`Forward`
      (`TimelineComponent.SetPlayRate` (`self.DoorTimeline`) (/ 1.0 (`KismetMathLibrary.FMax` (`self.CloseTime`) 0.008)) :!label _label_3)
      (`self.PlayTriggerSounds` false)
      (goto _label_2 :!via `Reverse`))
    (:`Backward`
      (goto _label))))

(event `self.TriggerOff`
  (params (TriggeringActor :type "Actor Object Reference") (Character :type "Character Object Reference"))
  (goto _label_3))

(event `self.ReceiveBeginPlay`
  (`parent.ReceiveBeginPlay`)
  (set `self.StartTransform` (`self.GetTransform`))
  (if (`self.StartOpen`)
    (set `self.Direction` "Forward")
    (`TimelineComponent.SetPlaybackPosition` (`self.DoorTimeline`) 1.0 false true)
    (goto _label_2)
    (else
      (set `self.Direction` "Backward"))))

(fn `OnUpdate`
  (params (Alpha :type "Float (double-precision)")))

(fn `UserConstructionScript`)