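; PB_TimerTrigger is a PuzzleBox trigger that dispatches its Actions once it has been active for a set Duration.
; Tick accumulates elapsed time, then on expiry sets Active to Repeat and calls StateChanged, either restarting or stopping the timer.
; StateChanged extends the parent, resetting time and playing sounds on activation or stopping them on deactivation.
; It also starts or stops the timer on the triggering character's PB_PlayerState.
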(event `self.ReceiveTick`
  (params (DeltaSeconds :type "Float (single-precision)"))
  (if (and (`self.Active`) (< (`self.ElapsedTime`) (`self.Duration`)))
    (bind _output_get (set `self.ElapsedTime` (+ DeltaSeconds (`self.ElapsedTime`))))
    (if (>= _output_get (`self.Duration`))
      (`self.Dispatch` (`self.Actions`) self)
      (set `self.Active` (`self.Repeat`))
      (`self.StateChanged`))))

(fn `StateChanged`
  (bind _triggeringcharacter (`self.TriggeringCharacter`))
  (`parent.StateChanged`)
  (if (`self.Active`)
    (set `self.ElapsedTime` 0.0)
    (`self.PlayTriggerSounds` true)
    (else
      (`self.StopTriggerSounds`)))
  (`/Engine/EditorBlueprintResources/StandardMacros.IsValid` _triggeringcharacter
    (:`Is Valid`
      (bind _aspb_player_state (cast `/Game/PuzzleBox/Blueprints/Private/PB_PlayerState` (`Pawn.PlayerState` _triggeringcharacter)))
      (if (`self.Active`)
        (`/Game/PuzzleBox/Blueprints/Private/PB_PlayerState.StartTimer` _aspb_player_state self)
        (else
          (`/Game/PuzzleBox/Blueprints/Private/PB_PlayerState.StopTimer` _aspb_player_state self))))))

(fn `UserConstructionScript`
  (`parent.UserConstructionScript`))