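; Area trigger that fires enter or exit actions as key actors move in and out of its overlap area.
; Begin and end overlap events filter actors through ActorIsKey, then raise or lower an overlap counter and share one dispatch check.
; Any change leaving the count above zero dispatches OnEnter, even a key leaving; otherwise it dispatches OnExit, passing the triggering actor.
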(event `self.ReceiveActorBeginOverlap`
  (params (OtherActor :type "Actor Object Reference"))
  (bind _otheractor (`self.OtherActor`))
  (bind _iskey (`self.Actor Is Key` OtherActor))
  (if _iskey
    (`/Engine/EditorBlueprintResources/StandardMacros.IncrementInt` (`self.KeyOverlapCount`)
      (:`  `
        (set `self.OtherActor` OtherActor)
        (if (> (`self.KeyOverlapCount`) 0) :!label _label
          (`self.Dispatch` (`self.OnEnter`) _otheractor)
          (else
            (`self.Dispatch` (`self.OnExit`) _otheractor)))))))

(event `self.ReceiveActorEndOverlap`
  (params (OtherActor :type "Actor Object Reference"))
  (bind _iskey (`self.Actor Is Key` OtherActor))
  (if _iskey
    (`/Engine/EditorBlueprintResources/StandardMacros.DecrementInt` (`self.KeyOverlapCount`)
      (:`  `
        (set `self.OtherActor` OtherActor)
        (goto _label)))))

(fn `UserConstructionScript`
  (`parent.UserConstructionScript`))