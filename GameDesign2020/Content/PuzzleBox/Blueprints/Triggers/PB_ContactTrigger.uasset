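; PB_ContactTrigger is a trigger Blueprint that fires its Actions when a key actor strikes its static mesh hard enough.
; On each component hit it checks the other actor with ActorIsKey, then compares the relative speed of both actors against MinimumSpeed.
; Impacts above that threshold dispatch Actions with the hitting actor as the triggering actor.
; An optional PrintSpeed flag prints the contact speed of key hits for tuning.
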(event `self.StaticMesh.OnComponentHit`
  (params (HitComponent :type "PrimitiveComponent Object Reference") (OtherActor :type "Actor Object Reference") (OtherComp :type "PrimitiveComponent Object Reference") (NormalImpulse :type "Vector Structure") (Hit :type "HitResult Structure (by ref)"))
  (bind _returnvalue (`KismetMathLibrary.VSize` (- (`self.GetVelocity` OtherActor) (`self.GetVelocity`))))
  (bind _iskey (`self.Actor Is Key` OtherActor))
  (if _iskey
    (if (`self.PrintSpeed`)
      (`KismetSystemLibrary.PrintString` (`KismetStringLibrary.Concat_StrStr` "Contact: " (`KismetStringLibrary.Conv_DoubleToString` _returnvalue))))
    (if (> _returnvalue (`self.MinimumSpeed`))
      (`self.Dispatch` (`self.Actions`) OtherActor))))

(fn `UserConstructionScript`
  (`parent.UserConstructionScript`))