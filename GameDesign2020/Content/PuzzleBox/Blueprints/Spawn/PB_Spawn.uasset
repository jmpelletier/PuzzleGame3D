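; PB_Spawn is a PuzzleBox actor that spawns an actor of a configurable class when triggered.
; On Triggeron, it checks the class is valid and spawns it at its own transform, adjusting for collisions but always spawning, with the triggering Character as instigator.
; It then plays trigger sounds and, if enabled, gives the spawned actor a limited life span.
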(event `self.TriggerOn`
  (params (TriggeringActor :type "Actor Object Reference") (Character :type "Character Object Reference"))
  (bind _spawnclass (`self.SpawnClass`))
  (if (`KismetSystemLibrary.IsValidClass` _spawnclass)
    (bind _returnvalue (`|SpawnActorFromClass` _spawnclass (`self.GetTransform`) "AdjustIfPossibleButAlwaysSpawn" "OverrideRootScale" null Character))
    (`self.PlayTriggerSounds` true)
    (if (`self.HasLifeSpan`)
      (`self.SetLifeSpan` _returnvalue (`self.LifeSpan`)))))

(fn `UserConstructionScript`
  (`parent.UserConstructionScript`))